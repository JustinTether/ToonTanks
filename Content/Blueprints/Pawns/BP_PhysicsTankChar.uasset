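; Physics-driven tank pawn that moves by applying forces and torques to its body and four wheels.
; Each Tick pushes the base mesh along its forward vector, scaled by the MoveForward axis.
; The sign of the Turn axis selects a side: positive torques both left wheels, negative both right wheels, around the body's right vector for skid-style steering.
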(event `self.ReceiveBeginPlay`)

(event `self.ReceiveTick`
  (params (DeltaSeconds :type "Float (single-precision)"))
  (bind _returnvalue (`self.GetInputAxisValue`))
  (bind _basemesh (`self.BaseMesh`))
  (bind _returnvalue_2 (`SceneComponent.GetRightVector` _basemesh))
  (bind _returnvalue_3 (* _returnvalue_2 (* _returnvalue 1000000.0)))
  (bind _returnvalue_4 (* _returnvalue_2 (* (* _returnvalue -1.0) 1000000.0)))
  (`PrimitiveComponent.AddForce` _basemesh (* (`SceneComponent.GetForwardVector` _basemesh) (* (`self.GetInputAxisValue`) 100000.0)) "None" false)
  (`/Engine/EditorBlueprintResources/StandardMacros.CompareFloat` _returnvalue
    (:`>`
      (`PrimitiveComponent.AddTorqueInRadians` (`self.WheelFL`) _returnvalue_3 "None" false)
      (`PrimitiveComponent.AddTorqueInRadians` (`self.WheelRL`) _returnvalue_3 "None" false))
    (:`<`
      (`PrimitiveComponent.AddTorqueInRadians` (`self.WheelFR`) _returnvalue_4 "None" false)
      (`PrimitiveComponent.AddTorqueInRadians` (`self.WheelRR`) _returnvalue_4 "None" false))))

(fn `UserConstructionScript`)