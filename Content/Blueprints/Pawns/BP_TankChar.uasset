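; Player tank pawn Blueprint that handles the escape menu and accumulates vertical aim input.
; Escape toggles a BP_EscapeMenu widget and the mouse cursor, creating a new widget each time it opens.
; Tick adds scaled axis input to AimY.
; A disconnected debug chain would print and draw a predicted projectile path from the spawn point's forward vector, AimY and ProjectileSpeed, but it never runs.
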(event `Key|Escape`
  (params (Key :type "Key Structure"))
  (bind _returnvalue (`GameplayStatics.GetPlayerController` 0))
  (:`Pressed`
    (if (`self.EscapeMenuVisible`)
      (`Widget.RemoveFromParent` (`self.EscapeMenu`))
      (set `self.EscapeMenuVisible` false)
      (set `PlayerController.bShowMouseCursor` false _returnvalue)
      (else
        (bind _returnvalue_2 (`|CreateWidget` "/Game/Blueprints/UI/BP_EscapeMenu.BP_EscapeMenu_C" _returnvalue))
        (bind _output_get (set `self.EscapeMenu` _returnvalue_2))
        (`UserWidget.AddToViewport` _output_get 0)
        (set `self.EscapeMenuVisible` true)
        (set `PlayerController.bShowMouseCursor` true _returnvalue)))))

(event `self.ReceiveTick`
  (params (DeltaSeconds :type "Float (single-precision)"))
  (set `self.AimY` (+ (`self.AimY`) (* (`self.GetInputAxisKeyValue`) 0.1))))

(fn `UserConstructionScript`)