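; GA_Fire is a gameplay ability that fires a projectile from a TankChar, ending immediately if the owner cannot fire.
; It spawns BP_ProjectileBase at the tank's spawn point, starts the fire delay and sets a fixed local forward velocity after writing the tank's ProjectileSpeed to InitialSpeed.
; The ability then waits for one Projectile.Hit gameplay event, and on authority applies GE_Damage to the payload's target data and ends.
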(event `self.K2_ActivateAbility`
  (bind _returnvalue_owneractor (break `GameplayAbilityActorInfo` (`self.GetActorInfo`)))
  (bind _astank_char (cast `TankChar` _returnvalue_owneractor)
    (:`then`
      (if (`TankChar.bCanFire` _astank_char)
        (bind _projectilespawnpoint (`TankChar.ProjectileSpawnPoint` _astank_char))
        (bind _returnvalue (`|SpawnActorFromClass` "/Game/Blueprints/BP_ProjectileBase.BP_ProjectileBase_C" (`KismetMathLibrary.MakeTransform` (`SceneComponent.K2_GetComponentLocation` _projectilespawnpoint) (`SceneComponent.K2_GetComponentRotation` _projectilespawnpoint)) "Undefined" "OverrideRootScale" _astank_char _astank_char))
        (bind _returnvalue_2 (`Actor.GetComponentByClass` _returnvalue "/Script/Engine.ProjectileMovementComponent"))
        (set `ProjectileMovementComponent.InitialSpeed` (`TankChar.ProjectileSpeed` _astank_char) _returnvalue_2)
        (`TankChar.SetFireDelay` _astank_char)
        (`ProjectileMovementComponent.SetVelocityInLocalSpace` _returnvalue_2 (1500.0 0.0 0.0))
        (bind (_asynctaskproxy _payload) (`AbilityTask_WaitGameplayEvent.WaitGameplayEvent` (struct :`TagName` "Projectile.Hit") null true)
          (:`then`
            (set `self.Async Task` _asynctaskproxy))
          (:`EventReceived`
            (`self.K2_HasAuthority`
              (:`True`
                (`self.BP_ApplyGameplayEffectToTarget` (`.TargetData` (break `GameplayEventData` _payload)) "/Game/Blueprints/GameplayAbilities/Effects/GE_Damage.GE_Damage_C")
                (`self.K2_EndAbility`)))))
        (else
          (`self.K2_EndAbility` :!label _label))))
    (:`CastFailed`
      (goto _label))))

(event `self.K2_OnEndAbility`
  (params (bWasCancelled :type Boolean))
  (`GameplayTask.EndTask` (`self.Async Task`)))