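; Functional test for tank movement that checks whether yaw input changes a player's view.
; PrepareTest creates and restarts a player, enables input on the first player's pawn, records the eye viewpoint and applies yaw input.
; It compares immediately in the same call, failing if location and rotation are both unchanged and succeeding otherwise.
; StartTest and Tick are unused, so the whole test runs during preparation.
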(event `self.ReceivePrepareTest`
  (bind _returnvalue (`GameplayStatics.CreatePlayer` -1))
  (`GameModeBase.RestartPlayer` (`GameplayStatics.GetGameMode`) _returnvalue)
  (`self.EnableInput` (`GameplayStatics.GetPlayerPawn` 0) _returnvalue)
  (bind (_outlocation _outrotation) (`self.GetActorEyesViewPoint` _returnvalue))
  (set `self.OriginalViewPoint` _outlocation)
  (set `self.OriginalViewRotation` _outrotation)
  (`PlayerController.AddYawInput` _returnvalue 200.0)
  (bind (_outlocation_2 _outrotation_2) (`self.GetActorEyesViewPoint` _returnvalue))
  (if (and (== (`self.OriginalViewPoint`) _outlocation_2) (== (`self.OriginalViewRotation`) _outrotation_2))
    (`self.FinishTest` "Failed")
    (else
      (`self.FinishTest` "Succeeded"))))

(fn `UserConstructionScript`)